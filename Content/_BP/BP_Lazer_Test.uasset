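; Test laser actor that fires a 500-unit visibility trace along a sphere component's forward vector, repeating through a Delay on Tick.
; Each pass moves the particle beam's end to the impact point, attaches a Leak emitter and generates a particle event.
; It also adds a new GameplayTasks component each pass to run a SpawnActor task for CupBP at the impact point, without checking for a hit.
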(event `self.ReceiveTick`
  (params (DeltaSeconds :type "Float (single-precision)"))
  (`KismetSystemLibrary.Delay` 0.2)
  (`self.lk`))

(event `lk`
  (bind _sphere (`self.Sphere`))
  (bind _particlesystem (`self.ParticleSystem`))
  (bind _returnvalue (`SceneComponent.K2_GetComponentLocation` _sphere))
  (bind _outhit (`KismetSystemLibrary.LineTraceSingle` :`Start` _returnvalue :`End` (+ _returnvalue (* (`KismetMathLibrary.GetForwardVector` (`SceneComponent.K2_GetComponentRotation` _sphere)) 500.0)) :`TraceChannel` "TraceTypeQuery1" :`TraceColor` (struct :`R` 0.829789 :`G` 1.0 :`A` 1.0) :`TraceHitColor` (struct :`R` 1.0 :`G` 1.0 :`B` 1.0 :`A` 1.0) :`DrawTime` 0.5))
  (bind _returnvalue_2 (`AddComponent|NODE_AddGameplayTasksComponent-0`))
  (bind (_bblockinghit _binitialoverlap _time _distance _location _impactpoint _normal _impactnormal _physmat _hitactor _hitcomponent _hitbonename _hititem _faceindex _tracestart _traceend) (`GameplayStatics.BreakHitResult` _outhit))
  (`ParticleSystemComponent.SetBeamEndPoint` _particlesystem 0 _impactpoint)
  (`GameplayStatics.SpawnEmitterAttached` "/Game/Playground/Particles/Leak/Leak.Leak" _particlesystem "None" _tracestart (struct) (1.0 1.0 1.0) "KeepRelativeOffset" true "AutoRelease")
  (`ParticleSystemComponent.GenerateParticleEvent` (`self.ParticleSystem`) "None" 5.0 _tracestart _impactpoint _traceend)
  (`GameplayTask_SpawnActor.SpawnActor` _returnvalue_2 _impactpoint (struct) "/Game/Playground/Objects/Cup/CupBP.CupBP_C" false null))

(fn `UserConstructionScript`)