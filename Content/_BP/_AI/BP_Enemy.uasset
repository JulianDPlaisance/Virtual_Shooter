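; BP_Enemy is an enemy actor that chases the player, deals damage at close range, and awards score when shot dead.
; A Delay-throttled Tick snaps its rotation toward the player, then either moves the capsule via MoveComponentTo or, within StoppingRadius, stops and deals damage.
; It finds BP_Global_Object on BeginPlay for player access and score updates.
; GotShot subtracts health, adding PointValue and destroying the actor at zero.
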(event `self.ReceiveBeginPlay`
  ;[1 1 1] On BeginPlay, find and set BP_Global_Object
  (bind _outactors (`GameplayStatics.GetAllActorsOfClass` "/Game/_BP/BP_Global_Object.BP_Global_Object_C"))
  (set `self.GlobalObject` (`|GetArrayItem` _outactors))
  (`self.RotateToPlayer`))

(event `KeepMoving`
  ;[1 1 1] Sets up movement and rotation over time to go towards the Player, and if it is close enough, stop moving, start hitting
  (`KismetSystemLibrary.MoveComponentTo` (`self.CapsuleComponent`) (stale `self.ReceiveTick` _outputrelativelocation) (stale `self.ReceiveTick` _outputrelativerotation) (stale `self.ReceiveTick` _easeout) (stale `self.ReceiveTick` _easein) (stale `self.ReceiveTick` _timetomoveover) :!label _label))

(event `StopMoving`
  ;[1 1 1] Sets up movement and rotation over time to go towards the Player, and if it is close enough, stop moving, start hitting
  (goto _label :!via `Stop`))

(event `self.ReceiveTick`
  (params (DeltaSeconds :type "Float (single-precision)"))
  ;[1 1 1] Try to execute every tick, limited by Delay
  (`KismetSystemLibrary.Delay` (`self.UpdateDelayTime`))
  ;[1 1 1] Creepy Sudden Rotation
  (`self.RotateToPlayer`)
  ;[1 1 1] Sets up movement and rotation over time to go towards the Player, and if it is close enough, stop moving, start hitting
  (bind (_outputrelativelocation _outputrelativerotation _easeout _easein _timetomoveover) (`self.MoveTowardsPlayer`))
  (if (`self.StayMoving`)
    (`self.KeepMoving`)
    (else
      (`self.StopMoving`))))

(event `GotShot`
  (params (Damage :type Integer))
  ;[1 1 1] If BP_Enemy gets shot, reduce health by damage, and if the damage makes TotalHealth <= 0 then update Global Score by PointValue and destroy this actor
  (bind _output_get (set `self.TotalHealth` (- (`self.TotalHealth`) Damage)))
  (if (<= _output_get 0)
    (`/Game/_BP/BP_Global_Object.UpdateGlobalScore` (`self.GlobalObject`) (`self.PointValue`))
    (`self.K2_DestroyActor`)))

(fn `DealDamage`
  (`/Game/_BP/BP_Main_Player.Receives_Damage` (`/Game/_BP/BP_Global_Object.Main_Player` (`self.GlobalObject`)) (`self.DamageCanDeal`)))

(fn `MoveTowardsPlayer`
  (returns (OutputRelativeLocation :type "Vector Structure") (OutputRelativeRotation :type "Rotator Structure") (EaseOut :type Boolean) (EaseIn :type Boolean) (TimeToMoveOver :type "Float (double-precision)"))
  (bind _returnvalue (`self.K2_GetActorLocation` (`/Game/_BP/BP_Global_Object.Main_Player` (`self.GlobalObject`))))
  (if (<= (`KismetMathLibrary.VSize` (- (`self.K2_GetActorLocation` self) _returnvalue)) (`self.StoppingRadius`))
    ;[1 1 1] If you are close enough, start the murderhobo time
    (`self.DealDamage`)
    (set `self.StayMoving` false)
    (else
      (set `self.StayMoving` true)
      (return _returnvalue (`self.K2_GetActorRotation` self) (`self.EaseIn?`) (`self.EaseOut?`) (`self.DeltaToCatchPlayer`)))))

(fn `RotateToPlayer`
  (`self.K2_SetActorRotation` self (`KismetMathLibrary.FindLookAtRotation` (`self.K2_GetActorLocation` self) (`self.K2_GetActorLocation` (`/Game/_BP/BP_Global_Object.Main_Player` (`self.GlobalObject`)))) false))

(fn `UserConstructionScript`)