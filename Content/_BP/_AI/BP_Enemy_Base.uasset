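; BP_Enemy_Base is an enemy actor that turns to face the player, takes shot damage and hurts the player on overlap.
; BeginPlay caches the first BP_Global_Object, which supplies the player reference for the per-tick look-at rotation.
; GotShot lowers Health and, at zero or below, destroys the enemy and sends PointValue to that object's score.
; Overlapping BP_Main_Player passes DamageToDeal to its ReceivesDamage.
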(event `self.ReceiveBeginPlay`
  ;[1 1 1] At Start, grab GlobalScore and set it's location to local GlobalScore
  (bind _outactors (`GameplayStatics.GetAllActorsOfClass` "/Game/_BP/BP_Global_Object.BP_Global_Object_C"))
  (set `self.globalScore` (`|GetArrayItem` _outactors)))

(event `GotShot`
  (params (Damage :type Integer))
  ;[1 1 1] If I getShot, lower my Health, if I go below or equal 0, destroy me and updaate Global Score
  (bind _output_get (set `self.Health` (- (`self.Health`) Damage)))
  (if (<= _output_get 0)
    (`self.K2_DestroyActor`)
    (`/Game/_BP/BP_Global_Object.UpdateGlobalScore` (`self.globalScore`) (`self.PointValue`))))

(event `self.ReceiveActorBeginOverlap`
  (params (OtherActor :type "Actor Object Reference"))
  ;[1 1 1] If I overlap with Main_Player, deal damage
  (bind _asbp_main_player (cast `/Game/_BP/BP_Main_Player` OtherActor))
  (`/Game/_BP/BP_Main_Player.Receives_Damage` _asbp_main_player (`self.DamageToDeal`)))

(event `self.ReceiveTick`
  (params (DeltaSeconds :type "Float (single-precision)"))
  (`self.RotateToPlayer`))

(fn `RotateToPlayer`
  (`self.K2_SetActorRotation` self (`KismetMathLibrary.FindLookAtRotation` (`self.K2_GetActorLocation` self) (`self.K2_GetActorLocation` (`/Game/_BP/BP_Global_Object.Main_Player` (`self.globalScore`)))) false))

(fn `UserConstructionScript`)