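; VR player hands Blueprint for a finger-gun shooter, handling firing, health, score and UI clicks.
; Shoot inputs set per-hand animation flags, play a sound and fire either a projectile or a debug-drawn line trace calling GotShot on steering actors.
; A face button swaps fire modes; another triggers pause by console command.
; Triggers click through widget interaction components, score lives on BP_Global_Object, and damage is gated by an invincibility flag.
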(event `self.ReceiveBeginPlay`
  ;[1 1 1] Grabs and sets Global Score, and updates ScoreText and HPText At the start of the game
  (bind _outactors (`GameplayStatics.GetAllActorsOfClass` "/Game/_BP/BP_Global_Object.BP_Global_Object_C"))
  (set `self.GlobalScore` (`|GetArrayItem` _outactors))
  (bind _outactors_2 (`GameplayStatics.GetAllActorsOfClass` "/Game/_BP/Menus_Widget.Menus_Widget_C"))
  (set `self.MenuUI` (`|GetArrayItem` _outactors_2))
  (`self.UpdateDamage` 0)
  (`self.UpdateScore` 0))

(event `RFire`
  (bind (_returnvalue_location _returnvalue_rotation) (`KismetMathLibrary.BreakTransform` (`SceneComponent.K2_GetComponentToWorld` (`self.RHandSpawnerSphere`))))
  ;[1 1 1] Right Fingergun Spawn Bullet
  (`self.RightFireProjectile` _returnvalue_location _returnvalue_rotation))

(event `LFire`
  (bind (_returnvalue_location _returnvalue_rotation) (`KismetMathLibrary.BreakTransform` (`SceneComponent.K2_GetComponentToWorld` (`self.LHandSpawnerSphere`))))
  ;[1 1 1] Left Fingergun Spawn Bullet
  (`self.LeftFireProjectile` _returnvalue_location _returnvalue_rotation))

(event `UpdateDamage`
  (params (`Damage To Deal` :type Integer))
  ;[1 1 1] Updates HP and HP Display on the Screen
  (set `self.Health` (- (`self.Health`) `Damage To Deal`)))

(event `Receives_Damage`
  (params (DamageToDeal :type Integer))
  ;[1 1 1] Should allow the player to take damage and grant invinciblity frames equal to Invincibility_Time
  (if (`self.bCanTakeDamage?`)
    (set `self.bCanTakeDamage?` false)
    (`self.UpdateDamage` DamageToDeal)
    (else
      (`KismetSystemLibrary.Delay` (`self.Invicibility_Time`))
      (set `self.bCanTakeDamage?` true))))

(event `UpdateScore`
  (params (ScoreAddition :type Integer))
  (bind _globalscore (`self.GlobalScore`))
  ;[1 1 1] Updates Score and Score Display on the Screen
  (set `/Game/_BP/BP_Global_Object.Score` (+ ScoreAddition (`/Game/_BP/BP_Global_Object.Score` _globalscore)) _globalscore))

(event `self.ReceiveTick`
  (params (DeltaSeconds :type "Float (single-precision)"))
  ;[1 1 1] Updates Score every 2 seconds
  (`KismetSystemLibrary.Delay` 0.1)
  (`self.UpdateScore` 0))

(event `Key|MotionController_Right_FaceButton2`
  (params (Key :type "Key Structure"))
  ;[1 1 1] The Logic for switching firing modes
  (:`Pressed`
    (switch `/Game/_Enums/EProjectileFireMode` (`self.FireMode`)
      (:`NewEnumerator0`
        (set `self.FireMode` "NewEnumerator1"))
      (:`NewEnumerator1`
        (set `self.FireMode` "NewEnumerator0")))))

(event `InputAction|LeftShoot` :paused true
  (params (Key :type "Key Structure"))
  ;[1 1 1] Shooting Fingerguns (Oculus Input and Animation)
  (:`Pressed`
    (if (not (`GameplayStatics.IsGamePaused`))
      (`|ExecutionSequence`
        (:`then_0`
          (set `self.IsLShooting` true)
          (`KismetSystemLibrary.Delay` 0.2)
          (set `self.IsLShooting` false))
        (:`then_1`
          (`|ExecutionSequence`
            (:`then_0`
              (`GameplayStatics.SpawnSoundAttached` (`self.fingergunpress`) (`self.LFGunAudio`) "None" (0.0 0.0 0.0) (struct) "KeepRelativeOffset" false 1.0 1.0 0.0 null null))
            (:`then_1`
              (`self.LFire`)))))))
  (:`Released`
    (set `self.IsLShooting` false)))

(event `InputAction|RightShoot` :paused true
  (params (Key :type "Key Structure"))
  ;[1 1 1] Shooting Fingerguns (Oculus Input and Animation)
  (:`Pressed`
    (if (not (`GameplayStatics.IsGamePaused`))
      (`|ExecutionSequence`
        (:`then_0`
          (set `self.IsRShooting` true)
          (`KismetSystemLibrary.Delay` 0.2)
          (set `self.IsRShooting` false))
        (:`then_1`
          (`|ExecutionSequence`
            (:`then_0`
              (`GameplayStatics.SpawnSoundAttached` (`self.fingergunpress`) (`self.RFGunAudio`) "None" (0.0 0.0 0.0) (struct) "KeepRelativeOffset" false 1.0 1.0 0.0 null null))
            (:`then_1`
              (`self.RFire`)))))))
  (:`Released`
    (set `self.IsRShooting` false)))

(event `Key|MotionController_Left_FaceButton2`
  (params (Key :type "Key Structure"))
  (:`Pressed`
    (`KismetSystemLibrary.ExecuteConsoleCommand` "ce PauseTheGame" null)))

(event `Key|LeftMouseButton`
  (params (Key :type "Key Structure"))
  (bind _lwidgetinteractioncomponent (`self.LWidgetInteractionComponent`))
  ;[1 1 1] Allows us to press UI Buttons
  (:`Pressed`
    (`WidgetInteractionComponent.PressPointerKey` _lwidgetinteractioncomponent "LeftMouseButton" :!label _label))
  (:`Released`
    (`WidgetInteractionComponent.ReleasePointerKey` _lwidgetinteractioncomponent "LeftMouseButton" :!label _label_2)))

(event `Key|MotionController_Left_Trigger`
  (params (Key :type "Key Structure"))
  ;[1 1 1] Allows us to press UI Buttons
  (:`Pressed`
    (goto _label))
  (:`Released`
    (goto _label_2)))

(event `Key|RightMouseButton`
  (params (Key :type "Key Structure"))
  (bind _rwidgetinteractioncomponent (`self.RWidgetInteractionComponent`))
  ;[1 1 1] Allows us to press UI Buttons
  (:`Pressed`
    (`WidgetInteractionComponent.PressPointerKey` _rwidgetinteractioncomponent "LeftMouseButton" :!label _label_3))
  (:`Released`
    (`WidgetInteractionComponent.ReleasePointerKey` _rwidgetinteractioncomponent "LeftMouseButton" :!label _label_4)))

(event `Key|MotionController_Right_Trigger`
  (params (Key :type "Key Structure"))
  ;[1 1 1] Allows us to press UI Buttons
  (:`Pressed`
    (goto _label_3))
  (:`Released`
    (goto _label_4)))

(fn `HittingUI`
  (`|ExecutionSequence`))

(fn `LeftFireProjectile`
  (params (SpawnLocation :type "Vector Structure") (SpawnRotator :type "Rotator Structure"))
  (bind _lhandendpoint (`self.LHandEndPoint`))
  (bind _returnvalue (`SceneComponent.K2_GetComponentLocation` _lhandendpoint))
  (switch `/Game/_Enums/EProjectileFireMode` (`self.FireMode`)
    (:`NewEnumerator0`
      (`|SpawnActorFromClass` "/Game/_BP/BP_Test_Projectile.BP_Test_Projectile_C" (`KismetMathLibrary.MakeTransform` SpawnLocation SpawnRotator) "AdjustIfPossibleButDontSpawnIfColliding" "OverrideRootScale" null null))
    (:`NewEnumerator1`
      (bind (_outhit _returnvalue_2) (`KismetSystemLibrary.LineTraceSingle` :`Start` _returnvalue :`End` (+ _returnvalue (* (`KismetMathLibrary.GetForwardVector` (`SceneComponent.K2_GetComponentRotation` _lhandendpoint)) 3000.0)) :`TraceChannel` "TraceTypeQuery2" :`DrawDebugType` "ForDuration" :`TraceColor` (struct :`R` 0.829789 :`G` 1.0 :`A` 1.0) :`TraceHitColor` (struct :`R` 1.0 :`G` 1.0 :`B` 1.0 :`A` 1.0) :`DrawTime` 0.5))
      (if _returnvalue_2
        (bind (_bblockinghit _binitialoverlap _time _distance _location _impactpoint _normal _impactnormal _physmat _hitactor _hitcomponent _hitbonename) (`GameplayStatics.BreakHitResult` _outhit))
        (if (== _hitbonename "Head")
          (bind _output_get (set `self.RHitActor` _hitactor))
          (bind _asmy_steering_actor_cpp (cast `/Game/_BP/_AI/MySteeringActor_CPP` _output_get))
          (`/Game/_BP/_AI/MySteeringActor_CPP.GotShot` _asmy_steering_actor_cpp 10)
          (else
            (bind _output_get_2 (set `self.RHitActor` _hitactor))
            (bind _asmy_steering_actor_cpp_2 (cast `/Game/_BP/_AI/MySteeringActor_CPP` _output_get_2))
            (`/Game/_BP/_AI/MySteeringActor_CPP.GotShot` _asmy_steering_actor_cpp_2 10)))))))

(fn `RightFireProjectile`
  (params (SpawnLocation :type "Vector Structure") (SpawnRotator :type "Rotator Structure"))
  (bind _rhandendpoint (`self.RHandEndPoint`))
  (bind _returnvalue (`SceneComponent.K2_GetComponentLocation` _rhandendpoint))
  (switch `/Game/_Enums/EProjectileFireMode` (`self.FireMode`)
    (:`NewEnumerator0`
      (`|SpawnActorFromClass` "/Game/_BP/BP_Test_Projectile.BP_Test_Projectile_C" (`KismetMathLibrary.MakeTransform` SpawnLocation SpawnRotator) "AdjustIfPossibleButDontSpawnIfColliding" "OverrideRootScale" null null))
    (:`NewEnumerator1`
      (bind (_outhit _returnvalue_2) (`KismetSystemLibrary.LineTraceSingle` :`Start` _returnvalue :`End` (+ _returnvalue (* (`KismetMathLibrary.GetForwardVector` (`SceneComponent.K2_GetComponentRotation` _rhandendpoint)) 3000.0)) :`TraceChannel` "TraceTypeQuery2" :`DrawDebugType` "ForDuration" :`TraceColor` (struct :`R` 0.829789 :`G` 1.0 :`A` 1.0) :`TraceHitColor` (struct :`R` 1.0 :`G` 1.0 :`B` 1.0 :`A` 1.0) :`DrawTime` 0.5))
      (if _returnvalue_2
        (bind (_bblockinghit _binitialoverlap _time _distance _location _impactpoint _normal _impactnormal _physmat _hitactor _hitcomponent _hitbonename) (`GameplayStatics.BreakHitResult` _outhit))
        (if (== _hitbonename "Head")
          (bind _output_get (set `self.RHitActor` _hitactor))
          (bind _asmy_steering_actor_cpp (cast `/Game/_BP/_AI/MySteeringActor_CPP` _output_get))
          (`/Game/_BP/_AI/MySteeringActor_CPP.GotShot` _asmy_steering_actor_cpp 10)
          (else
            (bind _output_get_2 (set `self.RHitActor` _hitactor))
            (bind _asmy_steering_actor_cpp_2 (cast `/Game/_BP/_AI/MySteeringActor_CPP` _output_get_2))
            (`/Game/_BP/_AI/MySteeringActor_CPP.GotShot` _asmy_steering_actor_cpp_2 10)))))))

(fn `UserConstructionScript`)