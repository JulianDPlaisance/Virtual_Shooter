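; VR player Blueprint with two finger guns, health and score text.
; Triggers or Q/E fire per hand, and a right-controller button toggles between spawned box projectiles and debug-drawn line-trace lasers that damage BP_Enemy, more for Head bone hits.
; Score lives on BP_Global_Object, found at BeginPlay, with its text refreshed through a delayed Tick.
; Damage clears CanTakeDamage, which only resets after a delay triggered by a subsequent hit.
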(event `self.ReceiveBeginPlay`
  ;[1 1 1] Grabs and sets Global Score, and updates ScoreText and HPText At the start of the game
  (bind _outactors (`GameplayStatics.GetAllActorsOfClass` "/Game/_BP/BP_Global_Object.BP_Global_Object_C"))
  (set `self.GlobalScore` (`|GetArrayItem` _outactors))
  (`self.UpdateDamage` 0)
  (`self.UpdateScore` 0))

(event `Key|MotionController_Right_FaceButton2`
  (params (Key :type "Key Structure"))
  (:`Pressed`
    (switch `/Game/_BP/ProjectileFireMode` (`self.FireMode`)
      (:`NewEnumerator0`
        (set `self.FireMode` "NewEnumerator1"))
      (:`NewEnumerator1`
        (set `self.FireMode` "NewEnumerator0")))))

(event `InputAxisKey|MotionController_Right_Thumbstick_X`
  (params (AxisValue :type "Float (single-precision)")))

(event `Key|E`
  (params (Key :type "Key Structure"))
  (bind (_returnvalue_location _returnvalue_rotation) (`KismetMathLibrary.BreakTransform` (`SceneComponent.K2_GetComponentToWorld` (`self.Sphere2`))))
  (:`Pressed`
    ;[1 1 1] Right Fingergun Spawn Bullet
    (`self.RightFireProjectile` _returnvalue_location _returnvalue_rotation :!label _label)))

(event `Key|Q`
  (params (Key :type "Key Structure"))
  (bind (_returnvalue_location _returnvalue_rotation) (`KismetMathLibrary.BreakTransform` (`SceneComponent.K2_GetComponentToWorld` (`self.Sphere1`))))
  (:`Pressed`
    ;[1 1 1] Left Fingergun Spawn Bullet
    (`self.LeftFireProjectile` _returnvalue_location _returnvalue_rotation :!label _label_2)))

(event `Key|MotionController_Right_Trigger`
  (params (Key :type "Key Structure"))
  ;[1 1 1] Right Fingergun Spawn Bullet
  (:`Pressed`
    (goto _label)))

(event `Key|MotionController_Left_Trigger`
  (params (Key :type "Key Structure"))
  ;[1 1 1] Left Fingergun Spawn Bullet
  (:`Pressed`
    (goto _label_2)))

(event `Receives_Damage`
  (params (DamageToDeal :type Integer))
  ;[1 1 1] Should allow the player to take damage and grant invinciblity frames equal to Invincibility_Time
  (if (`self.bCanTakeDamage?`)
    (set `self.bCanTakeDamage?` false)
    (`self.UpdateDamage` DamageToDeal)
    (else
      (`KismetSystemLibrary.Delay` (`self.Invicibility_Time`))
      (set `self.bCanTakeDamage?` true))))

(event `UpdateDamage`
  (params (`Damage To Deal` :type Integer))
  ;[1 1 1] Updates HP and HP Display on the Screen
  (bind _output_get (set `self.Health` (- (`self.Health`) `Damage To Deal`)))
  (`TextRenderComponent.K2_SetText` (`self.HealthText:`) (`|FormatText` "{Health_Text}: {HP_Amt}" (`KismetTextLibrary.Conv_StringToText` (`self.HealthString`)) _output_get)))

(event `self.ReceiveTick`
  (params (DeltaSeconds :type "Float (single-precision)"))
  ;[1 1 1] Updates Score every 2 seconds
  (`KismetSystemLibrary.Delay` 2.0)
  (`self.UpdateScore` 0))

(event `UpdateScore`
  (params (ScoreAddition :type Integer))
  (bind _globalscore (`self.GlobalScore`))
  ;[1 1 1] Updates Score and Score Display on the Screen
  (bind _output_get (set `/Game/_BP/BP_Global_Object.Score` (+ ScoreAddition (`/Game/_BP/BP_Global_Object.Score` _globalscore)) _globalscore))
  (`TextRenderComponent.K2_SetText` (`self.ScoreText:`) (`|FormatText` "{Score_Text}: {Score_Amt}" (`KismetTextLibrary.Conv_StringToText` (`self.ScoreString`)) _output_get)))

(fn `LeftFireProjectile`
  (params (SpawnLocation :type "Vector Structure") (SpawnRotation :type "Rotator Structure"))
  (bind _lgunendpoint (`self.LGunEndPoint`))
  (bind _returnvalue (`SceneComponent.K2_GetComponentLocation` _lgunendpoint))
  (switch `/Game/_BP/ProjectileFireMode` (`self.FireMode`)
    (:`NewEnumerator0`
      (`|SpawnActorFromClass` "/Game/_BP/BP_Test_Projectile.BP_Test_Projectile_C" (`KismetMathLibrary.MakeTransform` SpawnLocation SpawnRotation) "AdjustIfPossibleButDontSpawnIfColliding" "OverrideRootScale" null null))
    (:`NewEnumerator1`
      (bind (_outhit _returnvalue_2) (`KismetSystemLibrary.LineTraceSingle` :`Start` _returnvalue :`End` (+ _returnvalue (* (`KismetMathLibrary.GetForwardVector` (`SceneComponent.K2_GetComponentRotation` _lgunendpoint)) 3000.0)) :`TraceChannel` "TraceTypeQuery2" :`DrawDebugType` "Persistent" :`TraceColor` (struct :`R` 0.829789 :`G` 1.0 :`A` 1.0) :`TraceHitColor` (struct :`R` 1.0 :`G` 1.0 :`B` 1.0 :`A` 1.0)))
      (if _returnvalue_2
        (bind (_bblockinghit _binitialoverlap _time _distance _location _impactpoint _normal _impactnormal _physmat _hitactor _hitcomponent _hitbonename) (`GameplayStatics.BreakHitResult` _outhit))
        (if (== _hitbonename "Head")
          (bind _output_get (set `self.RHitActor` _hitactor))
          (bind _asbp_enemy (cast `/Game/_BP/_AI/BP_Enemy` _output_get))
          (`/Game/_BP/_AI/BP_Enemy.GotShot` _asbp_enemy 100)
          (else
            (bind _output_get_2 (set `self.RHitActor` _hitactor))
            (bind _asbp_enemy_2 (cast `/Game/_BP/_AI/BP_Enemy` _output_get_2))
            (`/Game/_BP/_AI/BP_Enemy.GotShot` _asbp_enemy_2 5)))))))

(fn `RightFireProjectile`
  (params (SpawnLocation :type "Vector Structure") (SpawnRotator :type "Rotator Structure"))
  (bind _rgunendpoint (`self.RGunEndPoint`))
  (bind _returnvalue (`SceneComponent.K2_GetComponentLocation` _rgunendpoint))
  (switch `/Game/_BP/ProjectileFireMode` (`self.FireMode`)
    (:`NewEnumerator0`
      (`|SpawnActorFromClass` "/Game/_BP/BP_Test_Projectile.BP_Test_Projectile_C" (`KismetMathLibrary.MakeTransform` SpawnLocation SpawnRotator) "AdjustIfPossibleButDontSpawnIfColliding" "OverrideRootScale" null null))
    (:`NewEnumerator1`
      (bind (_outhit _returnvalue_2) (`KismetSystemLibrary.LineTraceSingle` :`Start` _returnvalue :`End` (+ _returnvalue (* (`KismetMathLibrary.GetForwardVector` (`SceneComponent.K2_GetComponentRotation` _rgunendpoint)) 3000.0)) :`TraceChannel` "TraceTypeQuery2" :`DrawDebugType` "Persistent" :`TraceColor` (struct :`R` 0.829789 :`G` 1.0 :`A` 1.0) :`TraceHitColor` (struct :`R` 1.0 :`G` 1.0 :`B` 1.0 :`A` 1.0)))
      (if _returnvalue_2
        (bind (_bblockinghit _binitialoverlap _time _distance _location _impactpoint _normal _impactnormal _physmat _hitactor _hitcomponent _hitbonename) (`GameplayStatics.BreakHitResult` _outhit))
        (if (== _hitbonename "Head")
          (bind _output_get (set `self.RHitActor` _hitactor))
          (bind _asbp_enemy (cast `/Game/_BP/_AI/BP_Enemy` _output_get))
          (`/Game/_BP/_AI/BP_Enemy.GotShot` _asbp_enemy 100)
          (else
            (bind _output_get_2 (set `self.RHitActor` _hitactor))
            (bind _asbp_enemy_2 (cast `/Game/_BP/_AI/BP_Enemy` _output_get_2))
            (`/Game/_BP/_AI/BP_Enemy.GotShot` _asbp_enemy_2 5)))))))

(fn `UserConstructionScript`)