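; A grabbable dynamite stick with a spline fuse that a Flame actor can light, set up with fixed left- and right-hand grab transforms.
; A sphere overlap with a Flame activates the fuse fire effect, and Tick moves it along the Knot spline by elapsed time.
; When the spline's duration runs out, it spawns an explosion emitter and sound and destroys itself, applying no damage or force.
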(event `self.ReceiveTick`
  (params (DeltaSeconds :type "Float (single-precision)"))
  (if (`self.KnotLit`)
    (bind _output_get (set `self.KnotTime` (+ DeltaSeconds (`self.KnotTime`))))
    (if (> _output_get (`SplineComponent.Duration` (`self.Knot`)))
      (set `self.KnotLit` false)
      (`self.Explosion`)
      (else
        (`SceneComponent.K2_SetWorldLocation` (`self.KnotFIre`) (`SplineComponent.GetLocationAtTime` (`self.Knot`) (`self.KnotTime`) "World" false) false false)))))

(event `self.ReceiveBeginPlay`
  (bind _returnvalue (`KismetMathLibrary.MakeTransform` (2.1 0.2 9.7) (struct :`Pitch` 73.0 :`Yaw` 111.0 :`Roll` 178.0)))
  (`/Game/Framework/Hands/Grabable.SetFixedGrab` (`self.Grabable`) (`self.Dynamite`) _returnvalue "/Game/Framework/Hands/Model/Animations/Grabs/grab_round_medium.grab_round_medium" _returnvalue)
  (add `PrimitiveComponent.OnComponentBeginOverlap` (`self.Sphere`) (delegate `OnComponentBeginOverlap_Event_0`)))

(event `OnComponentBeginOverlap_Event_0`
  (params (OverlappedComponent :type "PrimitiveComponent Object Reference") (OtherActor :type "Actor Object Reference") (OtherComp :type "PrimitiveComponent Object Reference") (OtherBodyIndex :type Integer) (bFromSweep :type Boolean) (SweepResult :type "HitResult Structure (by ref)"))
  (cast `/Game/Playground/Objects/Flame/Flame` OtherActor)
  (if (not (`self.KnotLit`))
    (set `self.KnotLit` true)
    (`ActorComponent.Activate` (`self.KnotFIre`) false)))

(event `Explosion`
  (`GameplayStatics.SpawnEmitterAtLocation` "/Game/Playground/Particles/Grenades/Dynamite.Dynamite" (`self.K2_GetActorLocation`))
  (`self.K2_DestroyActor`)
  (`GameplayStatics.PlaySoundAtLocation` "/Game/Playground/Sounds/grenate.grenate" (`self.K2_GetActorLocation`)))

(fn `UserConstructionScript`)