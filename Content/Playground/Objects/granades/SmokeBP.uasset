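; SmokeBP is a grabbable smoke grenade that releases a smoke effect when triggered.
; BeginPlay sets a fixed grab pose for each hand and binds the Grabable release and GunFireHitTarget hit events.
; Release unlocks the grenade so a later impact detonates it, while gunfire detonates it even when still locked.
; Explode runs once, spawning the smoke emitter and playing explosion and steam sounds at the actor's location.
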(event `self.ReceiveBeginPlay`
  (bind _returnvalue (`KismetMathLibrary.MakeTransform` (3.2 1.2 8.2) (struct :`Pitch` 18.0 :`Yaw` 32.0 :`Roll` 107.0)))
  (bind _grabable (`self.Grabable`))
  (`/Game/Framework/Hands/Grabable.SetFixedGrab` _grabable (`self.GrenadeSmoke`) _returnvalue "/Game/Framework/Hands/Model/Animations/Grabs/hand_smoke.hand_smoke" _returnvalue)
  (add `/Game/Framework/Hands/Grabable.ReleaseNotify` _grabable (delegate `Unlock`)) ; Granade will be unlocked after grabbing it
  (add `/Game/Playground/BPs/GunFireHitTarget.Hit` (`self.GunFireHitTarget`) (delegate `GunFireHit`)))

(event `Unlock`
  (set `self.Unclocked` true))

(event `GunFireHit`
  (params (LocationLS :type "Vector Structure") (LocationWS :type "Vector Structure") (Normal :type "Vector Structure"))
  (`self.Explode`))

(event `self.ReceiveHit`
  (params (MyComp :type "PrimitiveComponent Object Reference") (Other :type "Actor Object Reference") (OtherComp :type "PrimitiveComponent Object Reference") (bSelfMoved :type Boolean) (HitLocation :type "Vector Structure") (HitNormal :type "Vector Structure") (NormalImpulse :type "Vector Structure") (Hit :type "HitResult Structure (by ref)"))
  (if (`self.Unclocked`)
    (`self.Explode`)))

(event `Explode`
  (if (not (`self.Exploded`))
    (set `self.Exploded` true)
    (`GameplayStatics.SpawnEmitterAtLocation` "/Game/Playground/Particles/Grenades/GrenadeSmoke.GrenadeSmoke" (`self.K2_GetActorLocation`) (`self.K2_GetActorRotation`))
    (`GameplayStatics.PlaySoundAtLocation` "/Game/Playground/Sounds/grenate.grenate" (`self.K2_GetActorLocation`) (struct) 0.2 0.5)
    (`GameplayStatics.PlaySoundAtLocation` "/Game/Playground/Sounds/steam.steam" (`self.K2_GetActorLocation`) (struct) 0.6)))

(fn `UserConstructionScript`)