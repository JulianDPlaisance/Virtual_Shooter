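; LighterBP is a grabbable lighter that produces a flame while the holder performs the thumb action.
; On BeginPlay it sets a fixed two-hand grab pose and hand animation on its Grabable component and binds thumb press and release to spawn and despawn events.
; Pressing spawns a Flame actor attached to the Scene point, keeping world rotation, and plays flicker and audio; releasing destroys the flame and stops the audio.
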(event `self.ReceiveBeginPlay`
  (bind _returnvalue (`KismetMathLibrary.MakeTransform` (1.1 -0.8 7.9) (struct :`Pitch` 73.599998 :`Yaw` 111.5 :`Roll` 178.600006)))
  (bind _grabable (`self.Grabable`))
  (`/Game/Framework/Hands/Grabable.SetFixedGrab` _grabable (`self.Lighter`) _returnvalue "/Game/Framework/Hands/Model/Animations/Grabs/hand_lighter.hand_lighter" _returnvalue)
  (add `/Game/Framework/Hands/Grabable.ThumbAction` _grabable (delegate `SpawnFlame`))
  (add `/Game/Framework/Hands/Grabable.ThumbActionStop` _grabable (delegate `DespawnFlame`)))

(event `SpawnFlame`
  (bind _returnvalue (`|SpawnActorFromClass` "/Game/Playground/Objects/Flame/Flame.Flame_C" (`KismetMathLibrary.MakeTransform` (0.0 0.0 0.0)) "Undefined" "OverrideRootScale" null null))
  (bind _output_get (set `self.FlameRef` _returnvalue))
  (`self.K2_AttachToComponent` _output_get (`self.Scene`) "None" "SnapToTarget" "KeepWorld" "KeepRelative" true)
  (`ActorComponent.Activate` (`self.Audio`) false)
  (`GameplayStatics.PlaySoundAtLocation` "/Game/Playground/Sounds/lighter_flicker.lighter_flicker" (`SceneComponent.K2_GetComponentLocation` (`self.Scene`)) (struct) 0.6))

(event `DespawnFlame`
  (bind _flameref (`self.FlameRef`))
  (`/Engine/EditorBlueprintResources/StandardMacros.IsValid` _flameref
    (:`Is Valid`
      (`self.K2_DestroyActor` _flameref)
      (`ActorComponent.Deactivate` (`self.Audio`)))))

(fn `UserConstructionScript`)