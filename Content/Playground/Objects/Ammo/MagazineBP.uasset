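; MagazineBP is a grabbable pistol magazine, with a Glock magazine volume, that holds a count of rounds.
; On BeginPlay it sets a fixed grab on that volume with a hand transform and grab animation.
; Round changes go through SetNumBullets, which clamps the count to capacity and refreshes the bullet meshes.
; Only two bullet meshes exist, shown when at least one or two rounds remain, also updated at construction.
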(event `self.ReceiveBeginPlay`
  (bind _returnvalue (`KismetMathLibrary.MakeTransform` (1.79 1.69 -0.3) (struct :`Pitch` 11.0 :`Yaw` -61.0 :`Roll` 171.0)))
  (`/Game/Framework/Hands/Grabable.SetFixedGrab` (`self.Grabable`) (`self.GlockMagazine`) _returnvalue "/Game/Framework/Hands/Model/Animations/Grabs/grab_brush.grab_brush" _returnvalue))

(fn `AddOrRemoveBullets`
  (params (AddAmmount :type Integer))
  (`self.SetNumBullets` (+ AddAmmount (`self.Rounds`))) ; Call to ensure clamping and everything else is consistent
)

(fn `AdjustBulletVisibility`
  (`SceneComponent.SetVisibility` (`self.Bullet1`) (>= (`self.Rounds`) 1) false)
  (`SceneComponent.SetVisibility` (`self.Bullet2`) (>= (`self.Rounds`) 2) false))

(fn `GetNumBullets`
  (returns (Value :type Integer))
  (return (`self.Rounds`)))

(fn `SetNumBullets`
  (params (`New Value` :type Integer))
  (set `self.Rounds` (`KismetMathLibrary.Clamp` `New Value` 0 15))
  (`self.AdjustBulletVisibility`))

(fn `UserConstructionScript`
  (`self.AdjustBulletVisibility`))