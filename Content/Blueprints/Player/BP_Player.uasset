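; BP_Player is a VR player Blueprint with a gun end point for each hand.
; Pressing the left or right motion controller trigger fires a straight 3000-unit line trace forward from that hand's gun end point on the Visibility channel.
; Both traces draw timed debug lines, and their hit results are not used, so shots have no gameplay effect here.
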(event `Key|MotionController_Left_Trigger`
  (params (Key :type "Key Structure"))
  (bind _lgunendpoint (`self.LGunEndPoint`))
  (bind _returnvalue (`SceneComponent.K2_GetComponentLocation` _lgunendpoint))
  (:`Pressed`
    (`KismetSystemLibrary.LineTraceSingle` :`Start` _returnvalue :`End` (+ _returnvalue (* (`KismetMathLibrary.GetForwardVector` (`SceneComponent.K2_GetComponentRotation` _lgunendpoint)) 3000.0)) :`TraceChannel` "TraceTypeQuery1" :`DrawDebugType` "ForDuration")))

(event `Key|MotionController_Right_Trigger`
  (params (Key :type "Key Structure"))
  (bind _rgunendpoint (`self.RGunEndPoint`))
  (bind _returnvalue (`SceneComponent.K2_GetComponentLocation` _rgunendpoint))
  (:`Pressed`
    (`KismetSystemLibrary.LineTraceSingle` :`Start` _returnvalue :`End` (+ _returnvalue (* (`KismetMathLibrary.GetForwardVector` (`SceneComponent.K2_GetComponentRotation` _rgunendpoint)) 3000.0)) :`TraceChannel` "TraceTypeQuery1" :`DrawDebugType` "ForDuration")))

(fn `UserConstructionScript`)